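; Game mode base for the Labyrinth game that runs the start, game-over and timeout flow.
; BeginPlay caches the StageController actor and creates start, HUD, end and timeout widgets.
; GameStart shows the start screen for a short delay with UI-only input, then swaps to the HUD and starts the stage.
; GameOver and Timeout briefly show their screens, soft-reset the stage and loop back into GameStart.
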(event `self.ReceiveBeginPlay`
  ;[1 1 1] Comment
  (`|ExecutionSequence`
    (:`then_0`
      (bind _outactors (`GameplayStatics.GetAllActorsOfClass` "/Game/Labyrinth/Blueprint/StageController.StageController_C"))
      (set `self.StageController` (`|GetArrayItem` _outactors)))
    (:`then_1`
      (bind _returnvalue (`|CreateWidget` "/Game/Labyrinth/Blueprint/WIdgetStart.WIdgetStart_C"))
      (set `self.Start_Display` _returnvalue)
      (bind _returnvalue_2 (`|CreateWidget` "/Game/Labyrinth/Blueprint/WidgetHud.WidgetHud_C"))
      (set `self.HeadsUp_Display` _returnvalue_2)
      (bind _returnvalue_3 (`|CreateWidget` "/Game/Labyrinth/Blueprint/WidgetEnd.WidgetEnd_C"))
      (set `self.Engame_Display` _returnvalue_3)
      (bind _returnvalue_4 (`|CreateWidget` "/Game/Labyrinth/Blueprint/WidgetTimeOut.WidgetTimeOut_C"))
      (set `self.TimeOut_Display` _returnvalue_4))))

(event `GameStart`
  (bind _returnvalue (`GameplayStatics.GetPlayerController` 0))
  (bind _start_display (`self.Start_Display`))
  ;[1 1 1] Gamestart
  (`UserWidget.AddToViewport` _start_display 0)
  (`WidgetBlueprintLibrary.SetInputMode_UIOnlyEx` _returnvalue null)
  (`KismetSystemLibrary.Delay` 2.0)
  (`Widget.RemoveFromParent` _start_display)
  (`UserWidget.AddToViewport` (`self.HeadsUp_Display`) 0)
  (`WidgetBlueprintLibrary.SetInputMode_GameOnly` _returnvalue)
  (`/Game/Labyrinth/Blueprint/StageController.GameStart` (`self.StageController`)))

(event `GameOver`
  (bind _engame_display (`self.Engame_Display`))
  ;[1 1 1] Gameover  on reset
  (`Widget.RemoveFromParent` (`self.HeadsUp_Display`))
  (`UserWidget.AddToViewport` _engame_display 0)
  (`KismetSystemLibrary.Delay` 2.0)
  (`Widget.RemoveFromParent` _engame_display)
  (`/Game/Labyrinth/Blueprint/StageController.SoftReset` (`self.StageController`))
  (`self.GameStart`))

(event `Timeout`
  (bind _timeout_display (`self.TimeOut_Display`))
  ;[1 1 1] Timeout Reset
  (`Widget.RemoveFromParent` (`self.HeadsUp_Display`))
  (`UserWidget.AddToViewport` _timeout_display 0)
  (`KismetSystemLibrary.RetriggerableDelay` 2.0)
  (`Widget.RemoveFromParent` _timeout_display)
  (`/Game/Labyrinth/Blueprint/StageController.SoftReset` (`self.StageController`))
  (`self.GameStart`))

(fn `UserConstructionScript`)
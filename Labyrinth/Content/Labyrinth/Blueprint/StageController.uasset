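; Stage controller for the Labyrinth game, tracking score, countdown, switches, pellets and best results for a stage.
; On BeginPlay it initializes counters and starts the game mode; GameStart runs a one-second looping timer that triggers Timeout at zero.
; GameOver converts remaining time into bonus score, updates records and UI strings, then notifies the game mode.
; SoftReset resets stage actors, respawns the player character and reinitializes the counters.
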(event `AddScore`
  (params (Score :type Integer))
  ;[1 1 1] Score
  (set `self.int_CurrentScore` (+ (`self.int_CurrentScore`) Score)))

(event `self.ReceiveBeginPlay`
  (bind _aslabyrinth_mode_base (cast `/Game/Labyrinth/Blueprint/LabyrinthModeBase` (`GameplayStatics.GetGameMode`)))
  (bind _output_get (set `self.GameMode` _aslabyrinth_mode_base))
  (`self.FSetupNewGame`)
  (`/Game/Labyrinth/Blueprint/LabyrinthModeBase.GameStart` _output_get))

(event `GameStart`
  (bind _returnvalue (`KismetSystemLibrary.K2_SetTimer` null "fElapsedTime" 1.0 true)))

(event `Timeout`
  ;[1 1 1] Comment
  (`KismetSystemLibrary.K2_ClearAndInvalidateTimerHandle` (stale `GameStart` _returnvalue))
  (`/Game/Labyrinth/Blueprint/LabyrinthModeBase.Timeout` (`self.GameMode`)))

(event `GameOver`
  (`|ExecutionSequence`
    (:`then_0`
      (`KismetSystemLibrary.K2_ClearAndInvalidateTimerHandle` (stale `GameStart` _returnvalue))
      (`self.AddScore` (* (`self.int_CurrentTime`) 50)))
    (:`then_1`
      (`self.fUpdate_IsBest`)
      (`self.fUpdateUI`))
    (:`then_2`
      (`/Game/Labyrinth/Blueprint/LabyrinthModeBase.GameOver` (`self.GameMode`)))))

(event `SwitchActivate`)

(event `SoftReset`
  ;[0 1 0.0201] SoftReset
  (`|ExecutionSequence`
    (:`then_0`
      (bind _outactors (`GameplayStatics.GetAllActorsOfClass` "/Game/Labyrinth/Blueprint/Actor_Switch.Actor_Switch_C"))
      (for _ _outactors
        (`self.SoftReset`)))
    (:`then_1`
      (bind _outactors_2 (`GameplayStatics.GetAllActorsOfClass` null))
      (for _ _outactors_2
        (`self.SoftReset`)))
    (:`then_2`
      (bind _outactors_3 (`GameplayStatics.GetAllActorsOfClass` "/Game/Labyrinth/Blueprint/Actor_Goal.Actor_Goal_C"))
      (`self.SoftReset`))
    (:`then_3`
      (bind _outactors_4 (`GameplayStatics.GetAllActorsOfClass` "/Game/Labyrinth/Blueprint/Actor_Goal.Actor_Goal_C"))
      (`self.SoftReset`))
    (:`then_4`
      ;[0 1 0.1711] Reset le joueur
      (bind _asthird_person_character (cast `/Game/ThirdPersonBP/Blueprints/ThirdPersonCharacter` (`GameplayStatics.GetPlayerCharacter` 0)))
      (`self.K2_DestroyActor` _asthird_person_character)
      (bind _returnvalue (`|SpawnActorFromClass` "/Game/ThirdPersonBP/Blueprints/ThirdPersonCharacter.ThirdPersonCharacter_C" (`self.Spawn_Point`) "Undefined" "OverrideRootScale" null null))
      (`Controller.Possess` (`Pawn.LastHitBy` (`GameplayStatics.GetPlayerCharacter` 0)) _returnvalue))
    (:`then_5`
      (`self.FSetupNewGame`))))

(fn `fElapsedTime`
  (bind _result (`/Engine/EditorBlueprintResources/StandardMacros.DecrementInt` (`self.int_CurrentTime`))
    (:`  `
      (`self.fUpdate_CurrentTime`)
      (if (<= _result 0)
        (`self.Timeout`)))))

(fn `FSetupNewGame`
  (`|ExecutionSequence`
    (:`then_0`
      (bind _outactors (`GameplayStatics.GetAllActorsOfClass` "/Game/Labyrinth/Blueprint/Actor_Switch.Actor_Switch_C"))
      (bind _output_get (set `self.int_SwitchLeft` (`KismetArrayLibrary.Array_Length` _outactors)))
      (set `self.int_CurrentTime` _output_get))
    (:`then_1`
      (set `self.int_CurrentTime` (`self.TIME_TOTAL`))
      (set `self.int_CurrentScore` 0)
      (set `self.int_PelletsCount` 0))))

(fn `fUpdate_CurrentTime`
  (set `self.String_CurrentTime` (`KismetStringLibrary.Conv_IntToString` (`self.int_CurrentTime`))))

(fn `fUpdate_IsBest`
  (bind _int_currenttime (`self.int_CurrentTime`))
  ;[1 1 1] BestSCore
  (`|ExecutionSequence`
    (:`then_0`
      (if (> (`self.int_CurrentScore`) (`self.int_BestScore`))
        (set `self.String_BestScore` "Best score")
        (set `self.int_BestScore` 0)
        (else
          (set `self.String_BestScore` ""))))
    (:`then_1`
      ;[1 1 1] BestTime
      (if (> _int_currenttime (`self.int_BestTime`))
        (set `self.String_IsBestTime` "Best time")
        (set `self.int_BestTime` _int_currenttime)
        (else
          (set `self.String_IsBestTime` ""))))))

(fn `fUpdate_PelletsCount`
  (set `self.String_PelletsCount` (`KismetStringLibrary.Concat_StrStr` (`KismetStringLibrary.Conv_IntToString` (`self.int_PelletsCount`)) "Collectable")))

(fn `fUpdate_SwitchRatio`
  (bind _int_switchleft (`self.int_SwitchLeft`))
  (set `self.String_SwitchesRatio` (`KismetStringLibrary.Concat_StrStr` (`KismetStringLibrary.Conv_IntToString` (- (`self.int_SwitchTotal`) _int_switchleft)) "/" (`KismetStringLibrary.Conv_IntToString` _int_switchleft))))

(fn `fUpdate_ToStrings`
  (bind _int_bestscore (`self.int_BestScore`))
  ;[0 1 0.06881] Comment
  (`|ExecutionSequence`
    (:`then_0`
      (set `self.String_CurrentScore` (`KismetStringLibrary.Conv_IntToString` (`self.int_CurrentScore`))))
    (:`then_1`
      (set `self.String_IsBestTime` (`KismetStringLibrary.Conv_IntToString` (`self.int_BestTime`))))
    (:`then_2`
      (if (<= _int_bestscore 0)
        (set `self.String_IsBestScore` "No score")
        (else
          (set `self.String_IsBestScore` (`KismetStringLibrary.Conv_IntToString` _int_bestscore)))))
    (:`then_3`
      (set `self.String_SwitchesTotal` (`KismetStringLibrary.Conv_IntToString` (`self.int_SwitchTotal`))))))

(fn `fUpdateUI`
  (`|ExecutionSequence`
    (:`then_0`
      (`self.fUpdate_SwitchRatio`))
    (:`then_1`
      (`self.fUpdate_SwitchRatio`))
    (:`then_2`
      (`self.fUpdate_SwitchRatio`))
    (:`then_3`
      (`self.fUpdate_SwitchRatio`))))

(fn `UserConstructionScript`)
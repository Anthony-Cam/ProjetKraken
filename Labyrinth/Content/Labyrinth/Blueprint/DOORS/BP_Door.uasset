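; BP_Door is a labyrinth door that slides vertically when the third-person character enters its trigger and slides back when they leave.
; Overlap events on CheckForPlayerTrigger drive two separate timelines, DoorSlide forward and Timeline_0 in reverse, whose scaled DoorAmount sets the Door's relative Z.
; Each timeline restarts from its endpoint, so an interrupted slide does not resume from the door's current position.
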(event `self.CheckForPlayerTrigger.OnComponentBeginOverlap`
  (params (OverlappedComponent :type "PrimitiveComponent Object Reference") (OtherActor :type "Actor Object Reference") (OtherComp :type "PrimitiveComponent Object Reference") (OtherBodyIndex :type Integer) (bFromSweep :type Boolean) (SweepResult :type "HitResult Structure (by ref)"))
  (cast `/Game/ThirdPersonBP/Blueprints/ThirdPersonCharacter` OtherActor)
  (if (not false)
    (bind (_direction _door_amount) (`Timeline|DoorSlide` :!via `PlayFromStart`)
      (:`Update`
        (`SceneComponent.K2_SetRelativeLocation` (`self.Door`) (`KismetMathLibrary.MakeVector` 0.0 0.0 (* _door_amount 80.0)) false false)))))

(event `self.CheckForPlayerTrigger.OnComponentEndOverlap`
  (params (OverlappedComponent :type "PrimitiveComponent Object Reference") (OtherActor :type "Actor Object Reference") (OtherComp :type "PrimitiveComponent Object Reference") (OtherBodyIndex :type Integer))
  (cast `/Game/ThirdPersonBP/Blueprints/ThirdPersonCharacter` OtherActor)
  (if (not false)
    (bind (_direction _door_amount) (`Timeline|Timeline_0` :!via `ReverseFromEnd`)
      (:`Update`
        (`SceneComponent.K2_SetRelativeLocation` (`self.Door`) (`KismetMathLibrary.MakeVector` 0.0 0.0 (* _door_amount 80.0)) false false)))))

(fn `UserConstructionScript`)
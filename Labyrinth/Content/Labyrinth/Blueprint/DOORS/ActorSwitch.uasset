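; ActorSwitch is a labyrinth switch that unlocks its linked door when something overlaps its collider.
; The overlap clears IsDoorLocked on MyDoor and plays a collapse sound at the switch.
; Every Tick, the switch mesh swaps between green and red materials based on IsActive, which this graph never sets.
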(event `self.ReceiveTick`
  (params (DeltaSeconds :type "Float (single-precision)"))
  (bind _switch (`self.Switch`))
  ;[1 1 1] Color
  (if (`self.IsActive`)
    (`PrimitiveComponent.SetMaterial` _switch 0 "/Game/Labyrinth/Blueprint/DOORS/GreenMat.GreenMat")
    (else
      (`PrimitiveComponent.SetMaterial` _switch 0 "/Game/Labyrinth/Blueprint/DOORS/RedMat.RedMat"))))

(event `self.SwitchCollider.OnComponentBeginOverlap`
  (params (OverlappedComponent :type "PrimitiveComponent Object Reference") (OtherActor :type "Actor Object Reference") (OtherComp :type "PrimitiveComponent Object Reference") (OtherBodyIndex :type Integer) (bFromSweep :type Boolean) (SweepResult :type "HitResult Structure (by ref)"))
  (set `/Game/Labyrinth/Blueprint/DOORS/BP_Door.IsDoorLocked` false (`self.MyDoor`))
  (`GameplayStatics.PlaySoundAtLocation` "/Game/StarterContent/Audio/Collapse_Cue.Collapse_Cue" (`SceneComponent.K2_GetComponentLocation` (`self.Switch`)) (struct) 1.0 1.0 0.0 null null null))

(fn `updateMateriel`)

(fn `UserConstructionScript`)
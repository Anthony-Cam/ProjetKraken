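; Labyrinth switch actor that shows a "Press B" prompt on box overlap while inactive and enables player input.
; Pressing B activates it once through a DoOnce, notifying StageController, tinting the button material and playing a sound.
; SoftReset clears the active state and re-arms the DoOnce, but reapplies the active colour.
; BeginPlay leaves StageController set to None, and end overlap neither hides the prompt nor disables input.
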(event `self.ReceiveBeginPlay`
  (bind _outactors (`GameplayStatics.GetAllActorsOfClass` "/Game/Labyrinth/Blueprint/StageController.StageController_C"))
  (set `self.StageController` null))

(event `self.Col_Button.OnComponentBeginOverlap`
  (params (OverlappedComponent :type "PrimitiveComponent Object Reference") (OtherActor :type "Actor Object Reference") (OtherComp :type "PrimitiveComponent Object Reference") (OtherBodyIndex :type Integer) (bFromSweep :type Boolean) (SweepResult :type "HitResult Structure (by ref)"))
  ;[1 1 1] Pour Afficher  Press B dans la box
  (set `self.B_isOverlapped` true)
  (`self.EnableInput` (`GameplayStatics.GetPlayerController` 0))
  (if (not (`self.b_IsActive`))
    (`SceneComponent.SetVisibility` (`self.Text_PressB`) (`self.B_isOverlapped`) false)))

(event `self.Col_Button.OnComponentEndOverlap`
  (params (OverlappedComponent :type "PrimitiveComponent Object Reference") (OtherActor :type "Actor Object Reference") (OtherComp :type "PrimitiveComponent Object Reference") (OtherBodyIndex :type Integer))
  ;[1 1 1] Pour Afficher  Press B dans la box
  (set `self.B_isOverlapped` true))

(event `Key|B`
  (params (Key :type "Key Structure"))
  ;[1 1 1] PressB
  (:`Pressed`
    (`self.Activate`)
    (`SceneComponent.SetVisibility` (`self.Text_PressB`) false false)))

(event `Activate`
  (`/Engine/EditorBlueprintResources/StandardMacros.DoOnce` false :!label _label
    (:`Completed`
      (`|ExecutionSequence`
        (:`then_0`
          (set `self.b_IsActive` true)
          (`/Game/Labyrinth/Blueprint/StageController.SwitchActivate` (`self.StageController`)))
        (:`then_1`
          (`MeshComponent.SetVectorParameterValueOnMaterials` (`self.Mesh_Button`) "Color_Activation" (`KismetMathLibrary.Conv_LinearColorToVector` (`self.Colour_Active`)))
          (`GameplayStatics.PlaySound2D` "/Game/StarterContent/Audio/Explosion01.Explosion01" 1.0 1.0 0.0 null null))))))

(event `SoftReset`
  ;[1 1 1] Reset
  (`|ExecutionSequence`
    (:`then_0`
      (set `self.b_IsActive` false)
      (`MeshComponent.SetVectorParameterValueOnMaterials` (`self.Mesh_Button`) "Color_Activation" (`KismetMathLibrary.Conv_LinearColorToVector` (`self.Colour_Active`))))
    (:`then_1`
      (goto _label :!via `Reset`))))

(fn `UserConstructionScript`)
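; Door actor for the Labyrinth project that responds to an Interact input while the player is nearby.
; A trigger volume enables the actor's input when the player character enters and disables it on exit.
; Pressing Interact plays DoorOppening, with no further opening logic in the graph.
; A SoftReset event restores the door's query and physics collision but sets its visibility to false.
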(event `self.TriggerVolume.OnComponentBeginOverlap`
  (params (OverlappedComponent :type "PrimitiveComponent Object Reference") (OtherActor :type "Actor Object Reference") (OtherComp :type "PrimitiveComponent Object Reference") (OtherBodyIndex :type Integer) (bFromSweep :type Boolean) (SweepResult :type "HitResult Structure (by ref)"))
  (if (== OtherActor (`GameplayStatics.GetPlayerCharacter` 0))
    (`self.EnableInput` (`GameplayStatics.GetPlayerController` 0))))

(event `InputAction|Interact`
  (params (Key :type "Key Structure"))
  (:`Pressed`
    (`Timeline|Door oppening`)))

(event `self.TriggerVolume.OnComponentEndOverlap`
  (params (OverlappedComponent :type "PrimitiveComponent Object Reference") (OtherActor :type "Actor Object Reference") (OtherComp :type "PrimitiveComponent Object Reference") (OtherBodyIndex :type Integer))
  (if (== OtherActor (`GameplayStatics.GetPlayerCharacter` 0))
    (`self.DisableInput` (`GameplayStatics.GetPlayerController` 0))))

(event `SoftReset`
  (bind _door (`self.Door`))
  (`PrimitiveComponent.SetCollisionEnabled` _door "QueryAndPhysics")
  (`SceneComponent.SetVisibility` _door false false))

(fn `UserConstructionScript`)
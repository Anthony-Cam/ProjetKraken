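; Labyrinth switch actor that opens its linked door when the player presses Q nearby.
; Actor overlap toggles input for the player, and the first Q press marks the switch active, recolors the button material, opens DoorRef and plays a sound.
; Separately, each character overlap with the button collider calls AddSwitch on the ThirdPersonCharacter, without requiring the key press.
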(event `self.Col_Button.OnComponentBeginOverlap`
  (params (OverlappedComponent :type "PrimitiveComponent Object Reference") (OtherActor :type "Actor Object Reference") (OtherComp :type "PrimitiveComponent Object Reference") (OtherBodyIndex :type Integer) (bFromSweep :type Boolean) (SweepResult :type "HitResult Structure (by ref)"))
  (bind _asthird_person_character (cast `/Game/ThirdPersonBP/Blueprints/ThirdPersonCharacter` OtherActor))
  (`/Game/ThirdPersonBP/Blueprints/ThirdPersonCharacter.Add Switch` _asthird_person_character)
  (`/Engine/EditorBlueprintResources/StandardMacros.DoOnce` true))

(event `Key|Q`
  (params (Key :type "Key Structure"))
  (:`Pressed`
    (`/Engine/EditorBlueprintResources/StandardMacros.DoOnce` false
      (:`Completed`
        (set `self.b_IsActive` true)
        (`MeshComponent.SetVectorParameterValueOnMaterials` (`self.Mesh_Button`) "None" (`KismetMathLibrary.Conv_LinearColorToVector` (`self.NewVar_0`)))
        (`/Game/Labyrinth/Projet1/Blueprint/Actor_Door.Open` (`self.DoorRef`))
        (`GameplayStatics.PlaySound2D` "/Engine/EditorSounds/GamePreview/EjectFromPlayer_Cue.EjectFromPlayer_Cue" 1.0 1.0 0.0 null null)))))

(event `self.ReceiveActorBeginOverlap`
  (params (OtherActor :type "Actor Object Reference"))
  (if (== OtherActor (`GameplayStatics.GetPlayerCharacter` 0))
    (`self.EnableInput` (`GameplayStatics.GetPlayerController` 0))))

(event `self.ReceiveActorEndOverlap`
  (params (OtherActor :type "Actor Object Reference"))
  (if (== OtherActor (`GameplayStatics.GetPlayerCharacter` 0))
    (`self.DisableInput` (`GameplayStatics.GetPlayerController` 0))))

(fn `UserConstructionScript`)
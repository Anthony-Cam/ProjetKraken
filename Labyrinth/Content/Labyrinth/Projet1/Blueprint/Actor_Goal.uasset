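; Goal actor for a labyrinth stage that ends the game when something overlaps its Goal component.
; On BeginPlay it caches the first StageController found in the level.
; The first overlap, with no check on the overlapping actor, hides the goal, plays a bird sound and calls GameOver on that controller.
; A DoOnce gate blocks repeat triggers until SoftReset shows the goal again and re-arms it.
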(event `self.ReceiveBeginPlay`
  (bind _outactors (`GameplayStatics.GetAllActorsOfClass` "/Game/Labyrinth/Projet1/StageController.StageController_C"))
  (set `self.StageController` (`|GetArrayItem` _outactors)))

(event `self.Goal.OnComponentBeginOverlap`
  (params (OverlappedComponent :type "PrimitiveComponent Object Reference") (OtherActor :type "Actor Object Reference") (OtherComp :type "PrimitiveComponent Object Reference") (OtherBodyIndex :type Integer) (bFromSweep :type Boolean) (SweepResult :type "HitResult Structure (by ref)"))
  (`/Engine/EditorBlueprintResources/StandardMacros.DoOnce` false :!label _label
    (:`Completed`
      (`SceneComponent.SetVisibility` (`self.Goal`) false false)
      (`GameplayStatics.PlaySound2D` "/Game/StarterContent/Audio/Starter_Birds01.Starter_Birds01" 1.0 1.0 0.0 null null)
      (`/Game/Labyrinth/Projet1/StageController.GameOver` (`self.StageController`)))))

(event `SoftReset`
  (`SceneComponent.SetVisibility` (`self.Goal`) true false)
  (goto _label :!via `Reset`))

(fn `UserConstructionScript`)